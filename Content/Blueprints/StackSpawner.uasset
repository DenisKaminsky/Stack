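; Spawner for a tile-stacking game that builds a starting tower, then spawns randomly colored tiles oscillating alternately along X and Y.
; Tick moves the current tile, reversing at a distance limit, until Space places it.
; Placement snaps near-aligned tiles within a tolerance, otherwise shrinks and recenters them to the overlap without spawning cut-off pieces.
; It then raises the spawner, spawns the next tile at that size and adds score through StackGameMode.
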(event Custom|SpawnTile
  (bind _leftspawner (Variables|Default|GetLeftSpawner))
  (bind _rightspawner (Variables|Default|GetRightSpawner))
  (bind _returnvalue (Transformation|GetWorldLocation _rightspawner))
  (bind _returnvalue_2 (Transformation|GetWorldLocation _leftspawner))
  (bind (_x _y _z) (Math|Vector|BreakVector _returnvalue_2))
  (bind (_x_2 _y_2 _z_2) (Math|Vector|BreakVector _returnvalue))
  (if (Variables|Default|GetIsOnLeft)
    (bind _returnvalue_3 (Game|SpawnActorfromClass "/Game/Blueprints/Tile.Tile_C" (Math|Transform|MakeTransform (Math|Vector|MakeVector _x (.Y (Math|Vector|BreakVector (Transformation|GetActorLocation (Variables|Default|GetPreviousTile)))) _z)) "Undefined" 0 0))
    (bind _output_get (Variables|Default|SetCurrentTile _returnvalue_3))
    (else
      (bind _returnvalue_4 (Game|SpawnActorfromClass "/Game/Blueprints/Tile.Tile_C" (Math|Transform|MakeTransform (Math|Vector|MakeVector (.X (Math|Vector|BreakVector (Transformation|GetActorLocation (Variables|Default|GetPreviousTile)))) _y_2 _z_2)) "Undefined" 0 0))
      (bind _output_get_2 (Variables|Default|SetCurrentTile _returnvalue_4))))
  (Transformation|SetActorScale3D _output_get (Transformation|GetActorScale3D (Variables|Default|GetPreviousTile)))
  (bind _rgbcolor (CallFunction|SetColor))
  (Rendering|Material|SetVectorParameterValueonMaterials (Variables|/Game/Blueprints/Tile.Tile_C|GetStaticMesh (Variables|Default|GetCurrentTile)) "BaseColor" _rgbcolor)
  (Variables|Default|SetCanMove true))

(event Custom|PlaceTile
  (bind _currenttile (Variables|Default|GetCurrentTile))
  (Variables|Default|SetCanMove false)
  (Transformation|AddWorldOffset (Variables|Default|GetDefaultSceneRoot) (Math|Vector|MakeVector 0.0 0.0 (Variables|Default|GetZvalue)) false false)
  (if (Variables|Default|GetIsOnLeft)
    (CallFunction|CalculateIntersectionLeft _currenttile (Variables|Default|GetPreviousTile))
    (Variables|Default|SetIsOnLeft false)
    (else
      (CallFunction|CalculateIntersectionRight _currenttile (Variables|Default|GetPreviousTile))
      (Variables|Default|SetIsOnLeft true)))
  (Variables|Default|SetPreviousTile (Variables|Default|GetCurrentTile))
  (CallFunction|SpawnTile)
  (bind _asstack_game_mode (Utilities|Casting|CastToStackGameMode (Game|GetGameMode)))
  (Default|AddScore _asstack_game_mode 1))

(event EventBeginPlay
  (for _index (range 0 (Variables|Default|GetNumberOfTilesToSpawn))
    (bind _returnvalue (Game|SpawnActorfromClass "/Game/Blueprints/Tile.Tile_C" (Transformation|GetWorldTransform (Variables|Default|GetDefaultSceneRoot)) "Undefined" 0 0))
    (bind _rgbcolor (CallFunction|SetColor))
    (Rendering|Material|SetVectorParameterValueonMaterials (Variables|/Game/Blueprints/Tile.Tile_C|GetStaticMesh _returnvalue) "BaseColor" _rgbcolor)
    (Transformation|AddWorldOffset (Variables|Default|GetDefaultSceneRoot) (Math|Vector|MakeVector 0.0 0.0 (Variables|Default|GetZvalue)) false false))
  (Variables|Default|SetPreviousTile _returnvalue)
  (CallFunction|SpawnTile))

(event EventTick
  (params (DeltaSeconds :type Float%20%28single-precision%29))
  (if (and (Variables|Default|GetCanMove) (Utilities|IsValid (Variables|Default|GetCurrentTile)))
    (CallFunction|MoveTile (Variables|Default|GetCurrentTile) DeltaSeconds (Variables|Default|GetTileSpeed))))

(event Input|KeyboardEvents|SpaceBar
  (params (Key :type Key%20Structure :default "None"))
  (:Pressed
    (CallFunction|PlaceTile)))

(fn ConstructionScript)

(fn MoveTile
  (params (CurrentTile :type Tile%20Object%20Reference) (DeltaTime :type Float%20%28single-precision%29) (Speed :type Float%20%28single-precision%29))
  (bind _returnvalue (* DeltaTime Speed))
  (if (Variables|Default|GetIsOnLeft)
    (bind _xwithdirection (CallFunction|AddDirectionX _returnvalue))
    (Transformation|AddActorWorldOffset CurrentTile (Math|Vector|MakeVector _xwithdirection 0.0 0.0))
    (else
      (bind _ywithdirection (CallFunction|AddDirectionY _returnvalue))
      (Transformation|AddActorWorldOffset CurrentTile (Math|Vector|MakeVector 0.0 _ywithdirection 0.0)))))

(fn CalculateIntersectionLeft
  (params (CurrentTile :type Tile%20Object%20Reference) (PrevTile :type Tile%20Object%20Reference))
  (bind _returnvalue (Transformation|GetActorScale3D CurrentTile))
  (bind _returnvalue_2 (Transformation|GetActorLocation CurrentTile))
  (bind _returnvalue_3 (Transformation|GetActorLocation CurrentTile))
  (bind (_x _y _z) (Math|Vector|BreakVector _returnvalue))
  (bind (_x_2 _y_2 _z_2) (Math|Vector|BreakVector _returnvalue_2))
  (bind (_x_3 _y_3 _z_3) (Math|Vector|BreakVector _returnvalue_3))
  (LocalVariables|SetCuurentTilePositionX (.X (Math|Vector|BreakVector (Transformation|GetActorLocation CurrentTile))))
  (LocalVariables|SetPrevTilePositionX (.X (Math|Vector|BreakVector (Transformation|GetActorLocation PrevTile))))
  (LocalVariables|SetPrevTileScaleX (.X (Math|Vector|BreakVector (Transformation|GetActorScale3D PrevTile))))
  (if (<= (Math|Float|Absolute(Float) (- (LocalVariables|GetCuurentTilePositionX) (LocalVariables|GetPrevTilePositionX))) (Variables|Default|GetTolerance))
    (Transformation|SetActorLocation CurrentTile (Math|Vector|MakeVector (LocalVariables|GetPrevTilePositionX) _y_3 _z_3) false false)
    (else
      (Transformation|SetActorScale3D CurrentTile (Math|Vector|MakeVector (- (LocalVariables|GetPrevTileScaleX) (Math|Float|Absolute(Float) (/ (- (LocalVariables|GetCuurentTilePositionX) (LocalVariables|GetPrevTilePositionX)) 1e+02))) _y _z))
      (Transformation|SetActorLocation CurrentTile (Math|Vector|MakeVector (/ (+ (LocalVariables|GetCuurentTilePositionX) (LocalVariables|GetPrevTilePositionX)) 2.0) _y_2 _z_2) false false))))

(fn CalculateIntersectionRight
  (params (CurrentTile :type Tile%20Object%20Reference) (PrevTile :type Tile%20Object%20Reference))
  (bind _returnvalue (Transformation|GetActorScale3D CurrentTile))
  (bind _returnvalue_2 (Transformation|GetActorLocation CurrentTile))
  (bind _returnvalue_3 (Transformation|GetActorLocation CurrentTile))
  (bind (_x _y _z) (Math|Vector|BreakVector _returnvalue))
  (bind (_x_2 _y_2 _z_2) (Math|Vector|BreakVector _returnvalue_2))
  (bind (_x_3 _y_3 _z_3) (Math|Vector|BreakVector _returnvalue_3))
  (LocalVariables|SetCuurentTilePositionY (.Y (Math|Vector|BreakVector (Transformation|GetActorLocation CurrentTile))))
  (LocalVariables|SetPrevTilePositionY (.Y (Math|Vector|BreakVector (Transformation|GetActorLocation PrevTile))))
  (LocalVariables|SetPrevTileScaleY (.Y (Math|Vector|BreakVector (Transformation|GetActorScale3D PrevTile))))
  (if (<= (Math|Float|Absolute(Float) (- (LocalVariables|GetCuurentTilePositionY) (LocalVariables|GetPrevTilePositionY))) (Variables|Default|GetTolerance))
    (Transformation|SetActorLocation CurrentTile (Math|Vector|MakeVector _x_3 (LocalVariables|GetPrevTilePositionY) _z_3) false false)
    (else
      (Transformation|SetActorScale3D CurrentTile (Math|Vector|MakeVector _x (- (LocalVariables|GetPrevTileScaleY) (Math|Float|Absolute(Float) (/ (- (LocalVariables|GetCuurentTilePositionY) (LocalVariables|GetPrevTilePositionY)) 1e+02))) _z))
      (Transformation|SetActorLocation CurrentTile (Math|Vector|MakeVector _x_2 (/ (+ (LocalVariables|GetCuurentTilePositionY) (LocalVariables|GetPrevTilePositionY)) 2.0) _z_2) false false))))

(fn AddDirectionX
  (params (x :type Float%20%28single-precision%29))
  (bind _currenttile (Variables|Default|GetCurrentTile))
  (bind _returnvalue (Transformation|GetActorLocation _currenttile))
  (bind _x (Math|Vector|BreakVector _returnvalue))
  (if (or (>= _x (LocalVariables|GetMaxDistance)) (<= _x (* (LocalVariables|GetMaxDistance) -1.0)))
    (bind _result (Utilities|NegateInt (Variables|Default|GetXDirection))
      (:%20%20
        (Variables|Default|SetXDirection _result))))
  (return (* (Variables|Default|GetXDirection) x)))

(fn AddDirectionY
  (params (Y :type Float%20%28single-precision%29))
  (bind _currenttile (Variables|Default|GetCurrentTile))
  (bind _returnvalue (Transformation|GetActorLocation _currenttile))
  (bind _y (Math|Vector|BreakVector _returnvalue))
  (if (or (>= _y (LocalVariables|GetMaxDistance)) (<= _y (* (LocalVariables|GetMaxDistance) -1.0)))
    (bind _result (Utilities|NegateInt (Variables|Default|GetYDirection))
      (:%20%20
        (Variables|Default|SetYDirection _result))))
  (return (* (Variables|Default|GetYDirection) Y)))

(fn SetColor
  (Variables|Default|SetH (Math|Random|RandomFloatinRange 0.0 3.5e+02))
  (Variables|Default|SetS (Math|Random|RandomFloatinRange 0.3 1.0))
  (Variables|Default|SetV (Math|Random|RandomFloatinRange 0.3 1.0))
  (return (Math|Vector|MakeVector (.r (Class|KismetMathLibrary|HSVtoRGB (Variables|Default|GetH) (Variables|Default|GetS) (Variables|Default|GetV) 1.0)) (.g (Class|KismetMathLibrary|HSVtoRGB (Variables|Default|GetH) (Variables|Default|GetS) (Variables|Default|GetV) 1.0)) (.b (Class|KismetMathLibrary|HSVtoRGB (Variables|Default|GetH) (Variables|Default|GetS) (Variables|Default|GetV) 1.0)))))